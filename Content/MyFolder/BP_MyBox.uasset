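; BP_MyBox is a networking debug Blueprint that displays replication state through two text elements.
; On BeginPlay it checks authority and sets AuthorityText to show whether this instance has it.
; Every Tick it rewrites VariableText with the current ReplicatedVar value, which nothing in these graphs modifies.
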(event EventBeginPlay
  ;[1 1 1] Authority Check
  (if (Ability|HasAuthority)
    (Rendering|Components|TextRender|SetText (Variables|Default|GetAuthorityText) (Utilities|Text|ToText(String) (Utilities|String|MakeLiteralString "Has Authority")))
    (else
      (Rendering|Components|TextRender|SetText (Variables|Default|GetAuthorityText) (Utilities|Text|ToText(String) (Utilities|String|MakeLiteralString "No Authority"))))))

(event EventTick
  (params (DeltaSeconds :type Float%20%28single-precision%29))
  ;[1 1 1] Replicated Variable
  (Rendering|Components|TextRender|SetText (Variables|Default|GetVariableText) (Utilities|Text|ToText(String) (Utilities|String|Append (Utilities|String|MakeLiteralString "ReplicatedVar: ") (Utilities|String|ToString(Float) (Variables|Default|GetReplicatedVar))))))

(fn ConstructionScript)